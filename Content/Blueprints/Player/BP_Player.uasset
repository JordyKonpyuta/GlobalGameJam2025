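; Player character for a bubble-pop rail shooter that rides a spline while the player looks around and shoots.
; Tick moves the capsule along the detached CharacterTrajectory at constant velocity, starting a one-time timer at the path's end, apparently to end the level through the game mode.
; Shooting spawns bullets from the camera using six-round ammo.
; Reloading scales with missing rounds, loops a sound, and updates the HUD created on BeginPlay.
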(event `EnhancedInput|/Game/Blueprints/Player/Controller/Inputs/IA_Shoot`
  (params (ActionValue :type Boolean) (ElapsedSeconds :type "Float (double-precision)") (TriggeredSeconds :type "Float (double-precision)") (InputAction :type "InputAction Object Reference" :default "/Game/Blueprints/Player/Controller/Inputs/IA_Shoot.IA_Shoot"))
  (bind _playercamera (`self.PlayerCamera`))
  (bind (_returnvalue_location _returnvalue_rotation _returnvalue_scale) (`KismetMathLibrary.BreakTransform` (`SceneComponent.K2_GetComponentToWorld` _playercamera)))
  ;[1 1 1] Gun Action
  ;;[1 1 1] Pew Pew
  (:`Started`
    (if (and (> (`self.BulletsRemaining`) 0) (not (`self.IsReloading`)))
      (`GameplayStatics.PlaySound2D` "/Game/SFX/SC_Shot.SC_Shot" 1.0 1.0 0.0 null null)
      (`|SpawnActorFromClass` "/Game/Blueprints/BP_Bullet.BP_Bullet_C" (`KismetMathLibrary.MakeTransform` (+ (* (`SceneComponent.GetForwardVector` _playercamera) 15.0) _returnvalue_location) _returnvalue_rotation _returnvalue_scale) "Undefined" "MultiplyWithRoot" null null)
      (bind _result (`/Engine/EditorBlueprintResources/StandardMacros.DecrementInt` (`self.BulletsRemaining`))
        (:`  `
          (`/Game/Blueprints/Widgets/WBP_HUD.SetBulletImage` (`self.HUD_Ref`) _result))))))

(event `EnhancedInput|/Game/Blueprints/Player/Controller/Inputs/IA_Rotato`
  (params (ActionValue :type "Vector2D Structure") (ElapsedSeconds :type "Float (double-precision)") (TriggeredSeconds :type "Float (double-precision)") (InputAction :type "InputAction Object Reference" :default "/Game/Blueprints/Player/Controller/Inputs/IA_Rotato.IA_Rotato"))
  ;[1 1 1] Player Looking Around
  (:`Triggered`
    (`self.AddControllerYawInput` ActionValue_X)
    (`self.AddControllerPitchInput` (* ActionValue_Y -1.0))))

(event `self.ReceiveBeginPlay`
  (bind _charactertrajectory (`self.CharacterTrajectory`))
  ;[1 1 1] Basically Begin Play
  (bind _output_get (set `self.CharacterTrajectoryRef` _charactertrajectory))
  (set `SplineComponent.Duration` (/ (`SplineComponent.GetSplineLength` _charactertrajectory) 500.0) _output_get)
  (`SceneComponent.K2_DetachFromComponent` (`self.CharacterTrajectory`) "KeepWorld" "KeepWorld" "KeepWorld" false)
  (bind _asbp_bubble_pop_game_mode (cast `/Game/Blueprints/GameBasics/BP_BubblePopGameMode` (`GameplayStatics.GetGameMode`)))
  (bind _output_get_2 (set `self.As BP Bubble Pop Game Mode` _asbp_bubble_pop_game_mode))
  (set `/Game/Blueprints/GameBasics/BP_BubblePopGameMode.PlayerRef` self _output_get_2)
  (`self.AddControllerYawInput` (`self.AddToRot(Yaw)`))
  (bind _returnvalue (`|CreateWidget` "/Game/Blueprints/Widgets/WBP_Stacks.WBP_Stacks_C"))
  (`UserWidget.AddToViewport` _returnvalue 0)
  (bind _returnvalue_2 (`CommonActivatableWidgetContainerBase.BP_AddWidget` (`/Game/Blueprints/Widgets/WBP_Stacks.CommonActivatableWidgetStack_34` _returnvalue) "/Game/Blueprints/Widgets/WBP_HUD.WBP_HUD_C"))
  (set `self.HUD_Ref` _returnvalue_2))

(event `EnhancedInput|/Game/Blueprints/Player/Controller/Inputs/IA_Reload`
  (params (ActionValue :type Boolean) (ElapsedSeconds :type "Float (double-precision)") (TriggeredSeconds :type "Float (double-precision)") (InputAction :type "InputAction Object Reference" :default "/Game/Blueprints/Player/Controller/Inputs/IA_Reload.IA_Reload"))
  (bind _bulletsremaining (`self.BulletsRemaining`))
  (bind _returnvalue (- 6 _bulletsremaining))
  (bind _returnvalue_2 (- 0.9 (* 0.05 _returnvalue)))
  (bind _returnvalue_3 (* _returnvalue _returnvalue_2))
  ;[1 1 1] Gun Action
  ;;[1 1 1] Reload
  (:`Started`
    (if (and (not (`self.IsReloading`)) (< _bulletsremaining 6))
      (set `self.IsReloading` true)
      (`/Game/Blueprints/Widgets/WBP_HUD.LaunchReload` (`self.HUD_Ref`) _returnvalue_3)
      (`KismetSystemLibrary.K2_SetTimerDelegate` (delegate `Reload All Bullets`) _returnvalue_3)
      (bind _returnvalue_4 (`KismetSystemLibrary.K2_SetTimerDelegate` (delegate `ReloadManualSound`) _returnvalue_2 true))
      (set `self.SoundEventTimer` _returnvalue_4)
      (`GameplayStatics.PlaySound2D` "/Game/SFX/SC_Reload.SC_Reload" 1.0 1.0 0.0 null null :!label _label))))

(event `ReloadManualSound`
  ;[1 1 1] Gun Action
  ;;[1 1 1] Reload
  (goto _label))

(event `Reload All Bullets`
  ;[1 1 1] Gun Action
  (bind _output_get (set `self.BulletsRemaining` 6))
  (`/Game/Blueprints/Widgets/WBP_HUD.SetBulletImage` (`self.HUD_Ref`) _output_get)
  (set `self.IsReloading` false)
  (`KismetSystemLibrary.K2_ClearAndInvalidateTimerHandle` (`self.SoundEventTimer`)))

(event `self.ReceiveTick`
  (params (DeltaSeconds :type "Float (single-precision)"))
  ;[1 1 1] Moving the Spline
  (bind _charactertrajectoryref (`self.CharacterTrajectoryRef`)
    (:`then`
      (bind _output_get (set `self.PositionInSpline` (+ (* DeltaSeconds (`self.SpeedModifier`)) (`self.PositionInSpline`))))
      (if (> _output_get (`SplineComponent.Duration` (`self.CharacterTrajectoryRef`)))
        (`/Engine/EditorBlueprintResources/StandardMacros.DoOnce` false
          (:`Completed`
            (`KismetSystemLibrary.K2_SetTimerDelegate` (`|CreateDelegate` :!event `level Ended`) 3.0)))
        (else
          (`SceneComponent.K2_SetRelativeLocation` (`self.CapsuleComponent`) (`SplineComponent.GetLocationAtTime` _charactertrajectoryref _output_get "World" true) false false))))
    (:`else`)))

(event `level Ended`
  (`/Game/Blueprints/GameBasics/BP_BubblePopGameMode.EndOfLevel` (`self.As BP Bubble Pop Game Mode`)))

(fn `UserConstructionScript`)