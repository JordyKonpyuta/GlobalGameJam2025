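; BP_Bubble is a shootable bubble target with multiple hit points, colour-coded by remaining HP.
; A looping timeline bobs and squash-stretches the mesh, while the construction script sets its starting material from HP.
; Bullet overlaps notify the manager, play a pop sound and HP-tinted Niagara burst, then decrement HP.
; Surviving bubbles swap material; depleted ones hide and set a timer for delayed removal.
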(event `self.ReceiveBeginPlay`
  ;[1 1 1] BeginPlay
  (`self.BubbleMovement`)
  ;[1 1 1] Debug
  (if (`self.TestSelfDestruct`)
    (`KismetSystemLibrary.Delay` 2.0)
    (`self.TestHit`)))

(event `BubbleMovement`
  ;[1 1 1] MovementLoop
  (bind (_direction _newtrack_0) (`Timeline|Movement` :!via `PlayFromStart`)
    (:`Update`
      (`SceneComponent.K2_SetRelativeLocation` (`self.BubbleMesh`) (`KismetMathLibrary.MakeVector` 0.0 0.0 (* _newtrack_0 10.0)) false false)
      (bind _returnvalue (/ _newtrack_0 10.0))
      (bind _returnvalue_2 (- 1.0 _returnvalue))
      (`SceneComponent.SetRelativeScale3D` (`self.BubbleMesh`) (`KismetMathLibrary.MakeVector` _returnvalue_2 _returnvalue_2 (+ 1.0 _returnvalue))))
    (:`Finished`
      (`self.BubbleMovement`))))

(event `self.ReceiveActorBeginOverlap`
  (params (OtherActor :type "Actor Object Reference"))
  (bind _managerref (`self.ManagerRef`))
  ;[1 1 1] TakeHit
  (cast `/Game/Blueprints/BP_Bullet` OtherActor :!label _label
    (:`then`
      (`/Engine/EditorBlueprintResources/StandardMacros.IsValid` _managerref
        (:`Is Valid`
          (`/Game/Blueprints/BP_BubbleManager.DamageNotification` _managerref)
          (`GameplayStatics.PlaySoundAtLocation` "/Game/SFX/SC_BubblePop.SC_BubblePop" (`self.K2_GetActorLocation`) (struct) 1.0 1.0 0.0 null null null null)
          (bind _returnvalue (`NiagaraFunctionLibrary.SpawnSystemAttached` "/Game/VFX/NS_BubblePop.NS_BubblePop" (`self.BubblePopEffect`) "None" (0.0 0.0 0.0) (struct) "KeepRelativeOffset" true false))
          (`FXSystemComponent.SetColorParameter` _returnvalue "BubbleColor" (select `int` (`self.HP`) :`0` (struct :`G` 0.356863 :`B` 1.0 :`A` 1.0) :`1` (struct :`G` 0.356863 :`B` 1.0 :`A` 1.0) :`2` (struct :`G` 1.0 :`B` 0.014911 :`A` 1.0) :`3` (struct :`R` 1.0 :`B` 0.095176 :`A` 1.0) :!type "LinearColor Structure"))
          (`ActorComponent.Activate` _returnvalue false)
          (bind _output_get (set `self.HP` (- (`self.HP`) 1)))
          (if (<= _output_get 0)
            (`SceneComponent.SetVisibility` (`self.BubbleMesh`) false true)
            (`KismetSystemLibrary.K2_SetTimerDelegate` (`|CreateDelegate` :!event `Death`) 1.5)
            (else
              (`self.ChangeMaterial`))))
        (:`Is Not Valid`
          (`KismetSystemLibrary.PrintString` "Cannot take damage: Manager is not valid!"))))
    (:`CastFailed`
      (`KismetSystemLibrary.PrintString` "That's not a bullet!"))))

(event `TestHit`
  ;[1 1 1] TakeHit
  (goto _label))

(event `Death`
  ;[1 1 1] Get Killededer
  (`self.K2_DestroyActor`))

(event `ChangeMaterial`
  ;[1 1 1] ChangeMaterial
  (`KismetSystemLibrary.PrintString` "Took damage, changing material")
  (`PrimitiveComponent.SetMaterial` (`self.BubbleMesh`) 0 (select `int` (`self.HP`) :`0` "/Game/Materials/M_Bubble3.M_Bubble3" :`1` "/Game/Materials/M_Bubble1.M_Bubble1" :`2` "/Game/Materials/M_Bubble2.M_Bubble2" :`3` "/Game/Materials/M_Bubble3.M_Bubble3" :!type "MaterialInterface Object Reference")))

(fn `UserConstructionScript`
  (`PrimitiveComponent.SetMaterial` (`self.BubbleMesh`) 0 (select `int` (`self.HP`) :`0` "/Game/Materials/M_Bubble3.M_Bubble3" :`1` "/Game/Materials/M_Bubble1.M_Bubble1" :`2` "/Game/Materials/M_Bubble2.M_Bubble2" :`3` "/Game/Materials/M_Bubble3.M_Bubble3" :!type "MaterialInterface Object Reference")))