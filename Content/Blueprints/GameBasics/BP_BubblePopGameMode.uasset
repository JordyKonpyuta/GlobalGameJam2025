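; Game mode for a bubble-popping game that presents the results screen when a level ends.
; BeginPlay caches the BP_PopGameInstance so the game mode can read the selected difficulty.
; EndOfLevel creates the WBP_EndLevel widget and fills in the popped percentage, popped count and total, which are not computed in this graph.
; The success or failure image depends on whether the percentage meets a difficulty-based threshold.
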(event `EndOfLevel`
  (bind _returnvalue (`|CreateWidget` "/Game/Blueprints/Widgets/WBP_EndLevel.WBP_EndLevel_C"))
  (`UserWidget.AddToViewport` _returnvalue 0)
  (`TextBlock.SetText` (`/Game/Blueprints/Widgets/WBP_EndLevel.Text_PercentageBubble` _returnvalue) (`|FormatText` "{p} %" (`self.Percentage`)))
  (`TextBlock.SetText` (`/Game/Blueprints/Widgets/WBP_EndLevel.Text_SmashedBubbles` _returnvalue) (`|FormatText` "Popped : {x}" (`self.SmashedBubbles`)))
  (`TextBlock.SetText` (`/Game/Blueprints/Widgets/WBP_EndLevel.Text_TotalBubbles` _returnvalue) (`|FormatText` "Total : {x}" (`self.TotalBubbles`)))
  (`Image.SetBrushFromTexture` (`/Game/Blueprints/Widgets/WBP_EndLevel.Image_Success` _returnvalue) (select `bool` (>= (`self.Percentage`) (select `int` (`/Game/Blueprints/GameBasics/BP_PopGameInstance.Difficulty` (`self.GameInstanceRef`)) :`0` 80.0 :`1` 90.0 :`2` 95.0)) :`false` "/Game/Assets/UI/T_Failure.T_Failure" :`true` "/Game/Assets/UI/T_Success.T_Success" :!type "Texture2D Object Reference") false))

(event `self.ReceiveBeginPlay`
  (bind _asbp_pop_game_instance (cast `/Game/Blueprints/GameBasics/BP_PopGameInstance` (`GameplayStatics.GetGameInstance`)))
  (set `self.GameInstanceRef` _asbp_pop_game_instance))

(fn `UserConstructionScript`)