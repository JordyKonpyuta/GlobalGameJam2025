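; Game instance for a bubble-pop game that holds the save object, mission scores, free-mode unlock and current level across maps.
; On Init it loads the existing save slot or attempts to write one, and Save writes scores and the unlock back.
; Levels open by index from an ordered array, with an outro cinematic widget past the last.
; Advancing first submits the game mode's percentage to the save object's best-score comparison.
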(event `self.ReceiveInit`
  (`self.Load/Create SaveFile`))

(event `Load Data`
  ;[1 1 1 1 45] SAVE PROCESS
  ;;[1 1 1 1 35] Load the Data
  (bind _save_game_object (`self.Save Game Object`)
    (:`then`
      (set `self.ScoreObtained/Missions` (`/Game/Blueprints/Saves/BP_Saves.ScoreObtained/Mission` _save_game_object))
      (set `self.Unlocked FreeMode` (`/Game/Blueprints/Saves/BP_Saves.UnlockedFreeMode` _save_game_object)))
    (:`else`
      (`KismetSystemLibrary.PrintString` "Data Corrupted"))))

(event `Save`
  ;[1 1 1 1 45] SAVE PROCESS
  ;;[1 1 1 1 35] Saving the Data
  (bind _save_game_object (`self.Save Game Object`)
    (:`then`
      (set `/Game/Blueprints/Saves/BP_Saves.ScoresToCompare` (`self.ScoreObtained/Missions`) _save_game_object)
      (`/Game/Blueprints/Saves/BP_Saves.Switch BestScore` _save_game_object)
      (set `/Game/Blueprints/Saves/BP_Saves.UnlockedFreeMode` (`self.Unlocked FreeMode`) _save_game_object)
      (`GameplayStatics.SaveGameToSlot` (`self.Save Game Object`) (`self.SaveName`)))
    (:`else`
      (bind _returnvalue (`GameplayStatics.LoadGameFromSlot` (`self.SaveName`)))
      (bind _asbp_saves (cast `/Game/Blueprints/Saves/BP_Saves` _returnvalue))
      (set `self.Save Game Object` _asbp_saves))))

(event `Unlocked FreePlay`
  ;[1 1 1 1 45] SAVE PROCESS
  ;;[1 1 1] You can now play as Luigi!
  (set `self.Unlocked FreeMode` true))

(event `Load/Create SaveFile`
  (bind _savename (`self.SaveName`))
  ;[1 1 1 1 45] SAVE PROCESS
  ;;[1 1 1 1 35] SaveFile Handling
  (bind _returnvalue (`GameplayStatics.DoesSaveGameExist` (`self.SaveName`)))
  (if _returnvalue
    (bind _returnvalue_2 (`GameplayStatics.LoadGameFromSlot` _savename))
    (bind _asbp_saves (cast `/Game/Blueprints/Saves/BP_Saves` _returnvalue_2))
    (set `self.Save Game Object` _asbp_saves)
    (`self.Load Data`)
    (else
      (`GameplayStatics.SaveGameToSlot` (`self.Save Game Object`) _savename))))

(event `LoadSameLevel`
  ;[1 1 1 1 45] LOADING LEVELS
  ;;[1 1 1 1 35] RELOAD : SAME LEVEL
  (`GameplayStatics.OpenLevelBySoftObjectPtr` (`|GetArrayItem` (`self.AllLevelsInOrder`) (`self.CurrentLevel`))))

(event `BackToMainMenu`
  ;[1 1 1 1 45] LOADING LEVELS
  ;;[1 1 1 1 35] LOAD : MAIN MENU
  (bind _output_get (set `self.CurrentLevel` 0))
  (`GameplayStatics.OpenLevelBySoftObjectPtr` (`|GetArrayItem` (`self.AllLevelsInOrder`) _output_get)))

(event `Load Specific Level`
  (params (LevelToLoad :type Integer))
  (bind _alllevelsinorder (`self.AllLevelsInOrder`))
  ;[1 1 1 1 45] LOADING LEVELS
  ;;[1 1 1 1 35] LOAD : A NEW LEVEL
  (set `self.CurrentLevel` LevelToLoad)
  (if (not (> (stale `LoadNextLevel` _result) (- (`KismetArrayLibrary.Array_Length` _alllevelsinorder) 1))) :!label _label
    (`GameplayStatics.OpenLevelBySoftObjectPtr` (`|GetArrayItem` _alllevelsinorder (stale `LoadNextLevel` _result)))
    (else
      (bind _returnvalue (`|CreateWidget` "/Game/Blueprints/Widgets/WBP_Cinematic.WBP_Cinematic_C"))
      (`UserWidget.AddToViewport` _returnvalue 0)
      (`/Game/Blueprints/Widgets/WBP_Cinematic.PlayOutro` _returnvalue))))

(event `LoadNextLevel`
  ;[1 1 1 1 45] LOADING LEVELS
  ;;[1 1 1 1 35] LOAD : A NEW LEVEL
  (`self.CheckIfScoreIsGood`)
  (bind _result (`/Engine/EditorBlueprintResources/StandardMacros.IncrementInt` (`self.CurrentLevel`))
    (:`  `
      (goto _label))))

(event `CheckIfScoreIsGood`
  (bind _asbp_bubble_pop_game_mode (cast `/Game/Blueprints/GameBasics/BP_BubblePopGameMode` (`GameplayStatics.GetGameMode`)))
  (bind _save_game_object (`self.Save Game Object`)
    (:`then`
      (`KismetArrayLibrary.Array_Set` (`/Game/Blueprints/Saves/BP_Saves.ScoresToCompare` _save_game_object) (`self.CurrentLevel`) (`/Game/Blueprints/GameBasics/BP_BubblePopGameMode.Percentage` _asbp_bubble_pop_game_mode))
      (`/Game/Blueprints/Saves/BP_Saves.Switch BestScore` _save_game_object))
    (:`else`)))