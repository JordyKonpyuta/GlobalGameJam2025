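; BP_BubbleManager tracks overall bubble-popping progress in the bubble pop game.
; On BeginPlay it sums the HP of every BP_Bubble in the level, registers itself as their manager, and reports the total to BP_BubblePopGameMode.
; Each damage notification decrements remaining HP, then updates the game mode's percentage and smashed count and the player HUD's bubble text.
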(event `self.ReceiveBeginPlay`
  ;[1 1 1] BeginPlay
  (bind _outactors (`GameplayStatics.GetAllActorsOfClass` "/Game/Blueprints/BP_Bubble.BP_Bubble_C"))
  (for _array_element _outactors
    (set `self.TotalHP` (+ (`self.TotalHP`) (`/Game/Blueprints/BP_Bubble.HP` _array_element)))
    (set `/Game/Blueprints/BP_Bubble.ManagerRef` self _array_element))
  (set `self.RemainingHP` (`self.TotalHP`))
  (bind _asbp_bubble_pop_game_mode (cast `/Game/Blueprints/GameBasics/BP_BubblePopGameMode` (`GameplayStatics.GetGameMode`)))
  (bind _output_get (set `self.GameModeRef` _asbp_bubble_pop_game_mode))
  (set `/Game/Blueprints/GameBasics/BP_BubblePopGameMode.TotalBubbles` (`self.TotalHP`) _output_get))

(event `DamageNotification`
  (bind _gamemoderef (`self.GameModeRef`))
  ;[1 1 1] ReduceTotalHP
  (set `self.RemainingHP` (- (`self.RemainingHP`) 1))
  (bind _output_get (set `self.Percentage` (- 100.0 (* (/ (`KismetMathLibrary.Conv_IntToDouble` (`self.RemainingHP`)) (`KismetMathLibrary.Conv_IntToDouble` (`self.TotalHP`))) 100.0))))
  (bind _output_get_2 (set `/Game/Blueprints/GameBasics/BP_BubblePopGameMode.Percentage` _output_get _gamemoderef))
  (`/Game/Blueprints/Widgets/WBP_HUD.SetBubbleText` (`/Game/Blueprints/Player/BP_Player.HUD_Ref` (`/Game/Blueprints/GameBasics/BP_BubblePopGameMode.PlayerRef` _gamemoderef)) _output_get_2)
  (set `/Game/Blueprints/GameBasics/BP_BubblePopGameMode.SmashedBubbles` (- (`self.TotalHP`) (`self.RemainingHP`)) _gamemoderef))

(fn `UserConstructionScript`)